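; ItemSalud is a health pickup actor that heals the character who overlaps it.
; On overlap it casts to the character Blueprint and reads that class's default Salud as the maximum health.
; If current Salud differs from that maximum, it adds MasSalud capped at the maximum and destroys itself.
; At full health the pickup is left in place.
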(event EventBeginPlay)

(event Collision|EventActorBeginOverlap
  (params (OtherActor :type Actor%20Object%20Reference))
  (bind _ascharacter (Utilities|Casting|CastTocharacter OtherActor))
  (if (not (== (.salud (Utilities|GetClassDefaults (Utilities|GetClass _ascharacter))) (Variables|/Game/Blueprints/character.character_C|Getsalud _ascharacter)))
    (Variables|/Game/Blueprints/character.character_C|Setsalud _ascharacter (Math|Float|Min(Float) (+ (Variables|/Game/Blueprints/character.character_C|Getsalud _ascharacter) (Variables|Default|Getmas%20salud)) (.salud (Utilities|GetClassDefaults (Utilities|GetClass _ascharacter)))))
    (Actor|DestroyActor)))

(event EventTick
  (params (DeltaSeconds :type Float%20%28single-precision%29)))

(fn ConstructionScript)