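; AI controller that hunts player-controlled characters and makes its pawn attack them.
; A looping timer runs ProcessAI, which finds a player character via a wide sphere overlap and keeps it as Target while valid.
; The pawn moves within primary attack range and calls AtaquePrimario on arrival, or roams to random navigable points when no target is found.
; A Jump event exists, but its timer is disconnected.
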(event Custom|Roam
  (bind _returnvalue (Pawn|GetControlledPawn))
  (Utilities|IsValid _returnvalue
    (:Is%20Valid
      (AI|AIMoveTo _returnvalue (.RandomLocation (Class|NavigationSystemV1|GetRandomPointinNavigableRadius (Transformation|GetActorLocation _returnvalue) 2e+03 0 0)) 0 5.0 false))))

(event Custom|Jump
  (bind _returnvalue (Pawn|GetControlledPawn))
  (Utilities|IsValid _returnvalue
    (:Is%20Valid
      (bind _ascharacter (Utilities|Casting|CastToCharacter _returnvalue))
      (Character|Jump _ascharacter))))

(event Custom|Process%20AI
  (bind _returnvalue (Pawn|GetControlledPawn))
  (Variables|Default|Gettarget
    (:then
      (AI|AIMoveTo _returnvalue "0, 0, 0" (Variables|Default|Gettarget) (Variables|/Game/Blueprints/character.character_C|GetRangoAtaquePrimario (.AsCharacter (Utilities|Casting|CastTocharacter _returnvalue))) false :!label _label
        (:OnSuccess
          (bind _ascharacter (Utilities|Casting|CastTocharacter (Pawn|GetControlledPawn)))
          (Default|AtaquePrimario _ascharacter))))
    (:else
      (bind _outactors (Collision|SphereOverlapActors "0, 0, 0" 1e+04 (Utilities|Array|MakeArray "ObjectTypeQuery3") 0 (Utilities|Array|MakeArray (Pawn|GetControlledPawn))))
      (bind _array_element (Utilities|Array|ForEachLoopwithBreak _outactors :!label _label_2)
        (:LoopBody
          (bind _ascharacter_2 (Utilities|Casting|CastTocharacter _array_element))
          (if (Class|Controller|IsPlayerController (Pawn|GetController _ascharacter_2))
            (Variables|Default|Settarget _ascharacter_2)
            (goto _label_2 Break)))
        (:Completed
          (Variables|Default|Gettarget
            (:then
              (goto _label))
            (:else
              (CallFunction|Roam))))))))

(event EventBeginPlay
  (Utilities|Time|SetTimerbyEvent (delegate Custom|Process%20AI) 2.0 true))

(event EventTick
  (params (DeltaSeconds :type Float%20%28single-precision%29)))

(fn ConstructionScript)