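; MR_Proyectil is a projectile Blueprint that damages characters it overlaps.
; On overlap it casts to the character class, ignores its own Instigator, applies fixed damage credited to the Instigator's controller, then destroys itself.
; The Destroyed event spawns an explosion particle effect at the actor's location, so the effect plays on any destruction.
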(event EventBeginPlay)

(event Collision|EventActorBeginOverlap
  (params (OtherActor :type Actor%20Object%20Reference))
  (bind _instigator (Variables|Actor|GetInstigator))
  (bind _ascharacter (Utilities|Casting|CastTocharacter OtherActor))
  (if (not (== _ascharacter _instigator))
    (Game|Damage|ApplyDamage _ascharacter 5e+01 (Pawn|GetController _instigator) self)
    (Actor|DestroyActor)))

(event EventTick
  (params (DeltaSeconds :type Float%20%28single-precision%29)))

(event EventDestroyed
  (Effects|SpawnEmitteratLocation "/Game/Blueprints/Effects/P_Explosion.P_Explosion" (Transformation|GetActorLocation)))

(fn ConstructionScript)