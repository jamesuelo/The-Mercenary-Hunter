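; GameMode that runs wave-based enemy spawning and ends the game after the last wave.
; Each wave's shuffled queue from OlaE feeds a looping timer that spawns AI at PlayerStarts, with location and rotation randomly picked separately.
; Enemy destruction triggers the next wave, broadcasting NuevaOla, once the queue and AIControllers are gone.
; After the final wave, the view blends to a MyCamera actor and the level restarts.
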(event Custom|Spawn
  (if (> (Utilities|Array|Length (Variables|Default|GetColaEnemigos)) 0)
    (bind _outactors (Actor|GetAllActorsOfClass "/Script/Engine.PlayerStart"))
    (bind _returnvalue (AI|SpawnAIFromClass (Utilities|Array|Get(acopy) (Variables|Default|GetColaEnemigos)) 0 (Transformation|GetActorLocation (Utilities|Array|Get(acopy) _outactors (Math|Random|RandomInteger (Utilities|Array|Length _outactors)))) (Transformation|GetActorRotation (Utilities|Array|Get(acopy) _outactors (Math|Random|RandomInteger (Utilities|Array|Length _outactors)))) false 0))
    (Utilities|Array|RemoveIndex (Variables|Default|GetColaEnemigos))
    (Game|BindEventtoOnDestroyed _returnvalue (delegate Custom|Comprobar%20Wave%20Compl))))

(event Custom|EmpezarWaveE
  (Math|Integer|IncrementInt (Variables|Default|Getindex)
    (:%20%20
      (Default|CallNuevaOla)
      (if (< (Utilities|Array|LastIndex (Variables|Default|GetOlaE)) (Variables|Default|Getindex))
        (CallFunction|FinJuego)
        (else
          (bind _output_get (Variables|Default|SetColaEnemigos (.olaenemigos (Utilities|Array|Get(acopy) (Variables|Default|GetOlaE) (Variables|Default|Getindex)))))
          (Utilities|Array|Shuffle _output_get))))))

(event Custom|Comprobar%20Wave%20Compl
  (params (DestroyedActor :type Actor%20Object%20Reference))
  (if (== (Utilities|Array|Length (Variables|Default|GetColaEnemigos)) 0)
    (bind _outactors (Actor|GetAllActorsOfClass "/Script/AIModule.AIController"))
    (if (== (Utilities|Array|Length _outactors) 0)
      (CallFunction|EmpezarwaveE))))

(event Custom|ResetJuego
  (Variables|Default|Setindex 0)
  (bind _output_get (Variables|Default|SetColaEnemigos (.olaenemigos (Utilities|Array|Get(acopy) (Variables|Default|GetOlaE) (Variables|Default|Getindex)))))
  (Utilities|Array|Shuffle _output_get))

(event Custom|fin%20Juego
  (bind _outactors (Actor|GetAllActorsOfClass "/Game/Blueprints/MyCamera.MyCamera_C"))
  (Game|Player|SetViewTargetwithBlend (Game|GetPlayerController 0) (Utilities|Array|Get(acopy) _outactors) 4.0 "VTBlend_Linear" 0.0 true)
  (Utilities|FlowControl|Delay 5.0)
  (Development|ExecuteConsoleCommand "restartlevel" 0))

(event EventBeginPlay
  (Utilities|Time|SetTimerbyEvent (delegate Custom|Spawn) 1.0 true)
  (CallFunction|ResetJuego))

(event EventTick
  (params (DeltaSeconds :type Float%20%28single-precision%29)))

(fn ConstructionScript)